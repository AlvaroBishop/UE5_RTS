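; BP_GameManager is a game manager in a test area that keeps a count of the units present in the level.
; Its Check event resets CurrentNumberOfUnits, then adds one for each actor found of AiCon_EnemyTriank, BP_Circlelry and BP_Cubet using GetAllActorsOfClass.
; Tick and the construction script are empty, and nothing in this graph calls Check or reads the count.
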(event Custom|Check
  (Variables|Default|SetCurrentNumberOfUnits 0)
  (bind _outactors (Actor|GetAllActorsOfClass "/Game/MyFirstRTS/Core/Enemy/AiCon_EnemyTriank.AiCon_EnemyTriank_C"))
  (for _array_element _outactors
    (Math|Integer|IncrementInt (Variables|Default|GetCurrentNumberOfUnits)))
  (bind _outactors_2 (Actor|GetAllActorsOfClass "/Game/MyFirstRTS/Core/Unit/BP_Circlelry.BP_Circlelry_C"))
  (for _array_element_2 _outactors_2
    (Math|Integer|IncrementInt (Variables|Default|GetCurrentNumberOfUnits)))
  (bind _outactors_3 (Actor|GetAllActorsOfClass "/Game/MyFirstRTS/Core/Unit/BP_Cubet.BP_Cubet_C"))
  (for _array_element_3 _outactors_3
    (Math|Integer|IncrementInt (Variables|Default|GetCurrentNumberOfUnits))))

(event EventTick
  (params (DeltaSeconds :type Float%20%28single-precision%29)))

(fn ConstructionScript)