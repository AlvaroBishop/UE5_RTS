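; RTS player controller handling camera panning, unit selection and orders, resource totals and building placement.
; Keys or screen-edge mouse scroll move the pawn, while a spawned marquee and click events fill the selection list.
; Action clicks sphere-test under the cursor, sending move, gather, interact or attack orders through interfaces by component found.
; In build mode, Tick moves a once-spawned building along a grid-snapped cursor trace until a selection click places it.
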(event Custom|AddActorSelectedToList
  (params (SelectedActor :type Actor%20Object%20Reference))
  (Utilities|Array|Add (Variables|Default|GetSelectedActors) SelectedActor)
  (Class|BPISelectionEvent|SelectThis(Message) SelectedActor))

(event Custom|DeselectAllActors
  (for _array_element (Variables|Default|GetSelectedActors)
    (if (Utilities|DoesObjectImplementInterface _array_element "/Game/MyFirstRTS/Core/Building/BPI_SelectionEvent.BPI_SelectionEvent_C")
      (Class|BPISelectionEvent|DeselectThis(Message) _array_element)))
  (Utilities|Array|Clear (Variables|Default|GetSelectedActors)))

(event Custom|Build
  ;[1 1 1] Comment
  (if (Variables|Build|GetisBuilding)
    (if (not (Variables|Default|GetcantBuild))
      (Variables|Build|SetisBuilding false)
      (Utilities|FlowControl|DoOnce false) ; enters at Reset
    )))

(event EventBeginPlay
  (bind _returnvalue (Game|SpawnActorfromClass "/Game/MyFirstRTS/Core/Player/BP_UnitSelectionMarquee.BP_UnitSelectionMarquee_C" (Math|Transform|MakeTransform "0, 0, 0" "0, 0, 0" "1.000000,1.000000,1.000000") "Undefined" "OverrideRootScale" 0 0))
  (Variables|Default|SetSelectionMarqueeRef _returnvalue))

(event EventTick
  (params (DeltaSeconds :type Float%20%28single-precision%29))
  ;[1 1 1] Comment
  (if (Variables|Build|GetisBuilding)
    (Utilities|FlowControl|Sequence
      (:then_0
        (Utilities|FlowControl|DoOnce false
          (:Completed
            (CallFunction|ChooseBuilding (stale _transform)))))
      (:then_1
        (bind _transform (CallFunction|Preview))
        (Transformation|SetActorLocation (Variables|Build|GetPreviewActor) (CallFunction|GridSnap) false false)))))

(event EventDeselectThisActor
  (params (ActorDeselected :type Actor%20Object%20Reference))
  (bind _returnvalue (Utilities|Array|RemoveItem (Variables|Default|GetSelectedActors) ActorDeselected))
  (if (and _returnvalue (Utilities|DoesObjectImplementInterface ActorDeselected "/Game/MyFirstRTS/Core/Building/BPI_SelectionEvent.BPI_SelectionEvent_C"))
    (Class|BPISelectionEvent|DeselectThis(Message) ActorDeselected)))

(event EventSelectThisActor
  (params (ActorSelected :type Actor%20Object%20Reference))
  (CallFunction|AddActorSelectedtoList ActorSelected))

(event EventClickSelectThisActor
  (params (ActorSelected :type Actor%20Object%20Reference))
  (Variables|Default|SetIsClickSelected true)
  (CallFunction|DeselectAllActors)
  (CallFunction|SelectThisActor ActorSelected))

(event Input|ActionEvents|InputActionMouseSelection
  (params (Key :type Key%20Structure :default "None"))
  (:Pressed
    (CallFunction|Build)
    (if (not (Variables|Default|GetIsClickSelected))
      (CallFunction|DeselectAllActors)
      (Transformation|SetActorLocation (Variables|Default|GetSelectionMarqueeRef) (.Location (Collision|BreakHitResult (.HitResult (Game|Player|GetHitResultUnderCursorbyChannel "TraceTypeQuery1" true)))) false false)
      (Default|StartResizingMarquee (Variables|Default|GetSelectionMarqueeRef))))
  (:Released
    (if (not (Variables|Default|GetIsClickSelected))
      (Default|EndResizingMarquee (Variables|Default|GetSelectionMarqueeRef))
      (else
        (Variables|Default|SetIsClickSelected false)))))

(event Input|ActionEvents|InputActionMouseAction
  (params (Key :type Key%20Structure :default "None"))
  (bind _hitresult (Game|Player|GetHitResultUnderCursorbyChannel "TraceTypeQuery1" true))
  (bind _location (Collision|BreakHitResult _hitresult))
  (:Released
    (if (Utilities|Array|IsNotEmpty (Variables|Default|GetSelectedActors))
      (bind _outactors (Collision|SphereOverlapActors (.Location (Collision|BreakHitResult (.HitResult (Game|Player|GetHitResultUnderCursorbyChannel "TraceTypeQuery1" true)))) 1e+02 (Utilities|Array|MakeArray "ObjectTypeQuery2" "ObjectTypeQuery3") 0))
      (if (Utilities|Array|IsEmpty _outactors)
        ;[1 1 1] Unit movement
        (for _array_element (Variables|Default|GetSelectedActors)
          (if (Utilities|DoesObjectImplementInterface _array_element "/Game/MyFirstRTS/Core/Unit/BPI_UnitActions.BPI_UnitActions_C")
            (Class|BPIUnitActions|MovetoThisLocation(Message) _array_element _location)
            (Niagara|SpawnSystematLocation "/Game/MyFirstRTS/Core/Player/NS_ClickIndicator.NS_ClickIndicator" _location)))
        (else
          (for _array_element_2 (Variables|Default|GetSelectedActors)
            (if (Utilities|DoesObjectImplementInterface _array_element_2 "/Game/MyFirstRTS/Core/Unit/BPI_UnitActions.BPI_UnitActions_C")
              (if (Utilities|IsValid (Actor|GetComponentbyClass (Utilities|Array|Get(acopy) _outactors) "/Game/MyFirstRTS/Core/Resource/BP_ResourceComponent.BP_ResourceComponent_C"))
                (Class|BPIUnitActions|GatherThisResource(Message) _array_element_2 (Utilities|Array|Get(acopy) _outactors))
                (elif (Utilities|IsValid (Actor|GetComponentbyClass (Utilities|Array|Get(acopy) _outactors) "/Game/MyFirstRTS/Core/Building/BP_BuildingComponent.BP_BuildingComponent_C"))
                  (Class|BPIUnitActions|InteractwithBuilding(Message) _array_element_2 (Utilities|Array|Get(acopy) _outactors))
                  (elif (Utilities|IsValid (Actor|GetComponentbyClass (Utilities|Array|Get(acopy) _outactors) "/Game/MyFirstRTS/Core/Unit/BP_UnitComponent.BP_UnitComponent_C"))
                    (if (Utilities|Enum|Equal(Enum) (Variables|/Game/MyFirstRTS/Core/Unit/BP_UnitComponent.BP_UnitComponent_C|GetTeamAttitude (Actor|GetComponentbyClass (Utilities|Array|Get(acopy) _outactors) "/Game/MyFirstRTS/Core/Unit/BP_UnitComponent.BP_UnitComponent_C")) "Hostile")
                      (Class|BPIUnitActions|AttackThisActor(Message) _array_element_2 (Utilities|Array|Get(acopy) _outactors)))))))))))))

(event Input|AxisEvents|InputAxisMoveForward
  (params (AxisValue :type Float%20%28single-precision%29))
  ;[1 1 1] Camera movement
  (Pawn|Input|AddMovementInput (Pawn|GetControlledPawn) (Math|Vector|GetForwardVector (Math|Rotator|MakeRotator 0.0 0.0 (.yaw (Pawn|GetControlRotation :!class /Script/Engine.Controller)))) (Math|Float|SelectFloat AxisValue (Variables|Default|GetMouseForwardScale) (!= AxisValue 0.0)) false))

(event Input|AxisEvents|InputAxisMoveRight
  (params (AxisValue :type Float%20%28single-precision%29))
  ;[1 1 1] Camera movement
  (Pawn|Input|AddMovementInput (Pawn|GetControlledPawn) (Math|Vector|GetRightVector (Math|Rotator|MakeRotator 0.0 0.0 (.yaw (Pawn|GetControlRotation :!class /Script/Engine.Controller)))) (Math|Float|SelectFloat AxisValue (Variables|Default|GetMouseRightScale) (!= AxisValue 0.0)) false))

(event Input|AxisEvents|InputAxisMouseMovement
  (params (AxisValue :type Float%20%28single-precision%29))
  (bind _locationy (Game|Player|GetMousePosition))
  (bind _returnvalue (Viewport|GetViewportSize))
  (bind _locationx (Game|Player|GetMousePosition))
  (bind _returnvalue_2 (Viewport|GetViewportSize))
  (bind _returnvalue_3 (/ _locationx (.x _returnvalue_2)))
  (bind _returnvalue_4 (/ _locationy (.y _returnvalue)))
  ;[1 1 1] Camera movement
  (Variables|Default|SetMouseRightScale (Math|Float|SelectFloat -1.0 (Math|Float|SelectFloat 1.0 0.0 (> _returnvalue_3 (- 1.0 (Variables|Default|GetViewportEdgeThreshold)))) (< _returnvalue_3 (Variables|Default|GetViewportEdgeThreshold))))
  (Variables|Default|SetMouseForwardScale (Math|Float|SelectFloat 1.0 (Math|Float|SelectFloat -1.0 0.0 (> _returnvalue_4 (- 1.0 (Variables|Default|GetViewportEdgeThreshold)))) (< _returnvalue_4 (Variables|Default|GetViewportEdgeThreshold)))))

(fn ConstructionScript)

(fn ReceiveResources
  (params (Type :type E_ResourceType%20Enum :default "NewEnumerator0") (Amount :type Integer))
  (Utilities|FlowControl|Sequence
    (:then_0
      (if (Utilities|Map|Contains (Variables|Default|GetStoredResources) Type)
        (Utilities|Map|Add (Variables|Default|GetStoredResources) Type (+ (.Value (Utilities|Map|Find (Variables|Default|GetStoredResources) Type)) Amount))
        (else
          (Utilities|Map|Add (Variables|Default|GetStoredResources) Type Amount))))
    (:then_1
      (bind _asbp_hud (Utilities|Casting|CastToBP_HUD (HUD|GetHUD)))
      (Default|UpdateResourceValue (Variables|/Game/MyFirstRTS/Core/Player/BP_HUD.BP_HUD_C|GetHUDWidgetRef _asbp_hud) Type (.Value (Utilities|Map|Find (Variables|Default|GetStoredResources) Type))))))

(fn Preview
  (bind _self self)
  (bind (_worldlocation _worlddirection) (Game|Player|ConvertMouseLocationToWorldSpace _self))
  (bind _outactors (Actor|GetAllActorswithTag "Building"))
  (bind _outhit (Collision|LineTraceByChannel _worldlocation (+ _worldlocation (* _worlddirection 1e+05)) "TraceTypeQuery1" false _outactors "None"))
  (if (!= (.HitActor (Collision|BreakHitResult _outhit)) 0)
    (Variables|Build|SetVectorGrid (.Location (Collision|BreakHitResult _outhit)))
    (return (Math|Transform|MakeTransform (.Location (Collision|BreakHitResult _outhit)) "0.000000,0.000000,0.000000"))))

(fn GridSnap
  (bind _vectorgrid (Variables|Build|GetVectorGrid))
  (return (Math|Vector|MakeVector (Math|Conversions|ToFloat(Integer) (* (/ (Math|Float|Floor (+ (.x _vectorgrid) 5e+01)) 1000) 1000)) (Math|Conversions|ToFloat(Integer) (* (/ (Math|Float|Floor (+ (.y _vectorgrid) 5e+01)) 1000) 1000)) (.z _vectorgrid))))

(fn ChooseBuilding
  (params (SpawnTransform :type Transform))
  (if (Variables|Build|GetisAttackTower)
    (bind _returnvalue (Game|SpawnActorfromClass "/Game/MyFirstRTS/Buildings/BP_House.BP_House_C" SpawnTransform "Undefined" "MultiplyWithRoot" 0 0))
    (Variables|Build|SetPreviewActor _returnvalue)
    (elif (Variables|Build|GetisHutTower)
      (bind _returnvalue_2 (Game|SpawnActorfromClass "/Game/MyFirstRTS/Buildings/BP_TrainingCenter.BP_TrainingCenter_C" SpawnTransform "Undefined" "MultiplyWithRoot" 0 0))
      (Variables|Build|SetPreviewActor _returnvalue_2)
      (elif (Variables|Build|GetisMineTower)
        (bind _returnvalue_3 (Game|SpawnActorfromClass "/Game/MyFirstRTS/Buildings/BP_TownHall.BP_TownHall_C" SpawnTransform "Undefined" "MultiplyWithRoot" 0 0))
        (Variables|Build|SetPreviewActor _returnvalue_3)))))

(fn GetTeamAttitude
  (return "Friendly"))