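; Attack tower building that damages units in its detection area, marked Hostile when flagged as enemy, and active after a short startup delay.
; Overlaps by BP_Cubet or BP_Circlelry refresh the overlapping-actor list, which toggles attacking and a Niagara effect above the tower.
; A DoOnce-gated recursive loop applies timed damage to the first listed actor, discarding invalid entries.
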(event OnComponentEndOverlap(DetectEnemy)
  (params (OverlappedComponent :type Primitive%20Component%20Object%20Reference) (OtherActor :type Actor%20Object%20Reference) (OtherComp :type Primitive%20Component%20Object%20Reference) (OtherBodyIndex :type Integer))
  (Utilities|Casting|CastToBP_Cubet OtherActor
    (:then
      _)
    (:CastFailed
      (Utilities|Casting|CastToBP_Circlelry OtherActor)))
  (Variables|Default|SetActorsOverlapping (Collision|GetOverlappingActors (Variables|Default|GetDetectEnemy) 0 :!class /Script/Engine.PrimitiveComponent))
  (if (Variables|Default|GetisSpawning)
    (CallFunction|CheckOverlapping)))

(event OnComponentBeginOverlap(DetectEnemy)
  (params (OverlappedComponent :type Primitive%20Component%20Object%20Reference) (OtherActor :type Actor%20Object%20Reference) (OtherComp :type Primitive%20Component%20Object%20Reference) (OtherBodyIndex :type Integer) (bFromSweep :type Boolean) (SweepResult :type Hit%20Result%20Structure%20%28by%20ref%29))
  (Utilities|Casting|CastToBP_Cubet OtherActor
    (:then
      _)
    (:CastFailed
      (Utilities|Casting|CastToBP_Circlelry OtherActor)))
  (Variables|Default|SetActorsOverlapping (Collision|GetOverlappingActors (Variables|Default|GetDetectEnemy) 0 :!class /Script/Engine.PrimitiveComponent))
  (if (Variables|Default|GetisSpawning)
    (CallFunction|CheckOverlapping)
    (CallFunction|Attacking)))

(event Custom|Attacking
  (bind _actorsoverlapping (Variables|Default|GetActorsOverlapping))
  (bind _output (Utilities|Array|Get(acopy) _actorsoverlapping))
  (Utilities|FlowControl|DoOnce false :!label _label
    (:Completed
      (if (Variables|Default|GetisAttacking)
        (Utilities|IsValid _output
          (:Is%20Valid
            (Game|Damage|ApplyDamage _output 1e+01 0 0)
            (Utilities|FlowControl|Delay 1.0)
            (Utilities|FlowControl|Sequence
              (:then_0
                (CallFunction|ResetAttacking))
              (:then_1
                (CallFunction|Attacking))))
          (:Is%20Not%20Valid
            (Utilities|Array|RemoveIndex (Variables|Default|GetActorsOverlapping))
            (CallFunction|Attacking)))
        (else
          (goto _label Reset))))))

(event Custom|ResetAttacking
  (bind _actorsoverlapping (Variables|Default|GetActorsOverlapping))
  (bind _output (Utilities|Array|Get(acopy) _actorsoverlapping))
  (Utilities|FlowControl|DoOnce false) ; enters at Reset
)

(event EventBeginPlay
  (|CallParentFunction)
  (Utilities|FlowControl|Delay 3.0)
  (Variables|Default|SetisSpawning true)
  (if (Variables|Default|GetisEnemy)
    (Variables|/Game/MyFirstRTS/Core/Building/BP_BuildingComponent.BP_BuildingComponent_C|SetTeamAttitude (Variables|Default|GetBP_BuildingComponent) "Hostile")))

(event Collision|EventActorBeginOverlap
  (params (OtherActor :type Actor%20Object%20Reference))
  (|CallParentFunction OtherActor) ; This node is disabled and will not be called.\nDrag off pins to build functionality.
)

(event EventTick
  (params (DeltaSeconds :type Float%20%28single-precision%29))
  (|CallParentFunction DeltaSeconds)
  (Utilities|FlowControl|Delay 3.0))

(event EventBuildingClicked
  (|CallParentFunction)
  (Development|PrintString "Statue clicked"))

(fn ConstructionScript
  (|CallParentFunction))

(fn CheckOverlapping
  (if (Utilities|Array|IsEmpty (Variables|Default|GetActorsOverlapping))
    (Variables|Default|SetisAttacking false)
    (bind _particles (Variables|Default|GetParticles)
      (:then
        (Components|DestroyComponent _particles))
      (:else))
    (elif (not (Variables|Default|GetisAttacking))
      (Variables|Default|SetisAttacking true)
      (bind _returnvalue (Niagara|SpawnSystematLocation "/Game/PaulTestArea/Damage.Damage" (+ (Transformation|GetActorLocation) "0.000000,0.000000,300.000000")))
      (Variables|Default|SetParticles _returnvalue))))