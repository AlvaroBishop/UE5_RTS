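; BP_Hut is a house building that contributes a fixed number of units to the game manager's NumberOfUnits while it stands.
; On BeginPlay it finds and caches BP_GameManager, then raises that count.
; When its BP_BuildingComponent reports destruction, it subtracts the same amount and prints a debug message.
; Clicking it runs the parent building's click handling, then prints a debug string.
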(event OnBuildingDestroyed(BP_BuildingComponent)
  (params (TeamAttitude :type ETeamAttitude%20Enum :default "Friendly"))
  (bind _gamemanager (Variables|Default|GetGameManager))
  (Variables|/Game/PaulTestArea/BP_GameManager.BP_GameManager_C|SetNumberOfUnits _gamemanager (- (Variables|/Game/PaulTestArea/BP_GameManager.BP_GameManager_C|GetNumberOfUnits _gamemanager) 5))
  (Development|PrintString "-Units"))

(event EventBeginPlay
  (bind _returnvalue (Actor|GetActorOfClass "/Game/PaulTestArea/BP_GameManager.BP_GameManager_C"))
  (bind _output_get (Variables|Default|SetGameManager _returnvalue))
  (Variables|/Game/PaulTestArea/BP_GameManager.BP_GameManager_C|SetNumberOfUnits _output_get (+ (Variables|/Game/PaulTestArea/BP_GameManager.BP_GameManager_C|GetNumberOfUnits _returnvalue) 5)))

(event Collision|EventActorBeginOverlap
  (params (OtherActor :type Actor%20Object%20Reference)))

(event EventTick
  (params (DeltaSeconds :type Float%20%28single-precision%29)))

(event EventBuildingClicked
  (|CallParentFunction)
  (Development|PrintString "House clicked"))

(fn ConstructionScript
  (|CallParentFunction))