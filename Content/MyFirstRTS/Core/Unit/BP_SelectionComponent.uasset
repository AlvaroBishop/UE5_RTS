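; BP_SelectionComponent is a unit component for an RTS that provides a decal-based selection indicator on its owning actor.
; On BeginPlay it adds a rotated decal component to the owner, applies the selection indicator material and starts it hidden.
; It sizes the decal from IndicatorRadius relative to the decal's extents and positions it at IndicatorOffset.
; Show and Hide events toggle the decal's visibility and hidden-in-game state.
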(event Custom|HideSelectionDecal
  (bind _decalcompref (Variables|Default|GetDecalCompRef))
  (Rendering|SetVisibility _decalcompref false false)
  (Development|SetHiddeninGame _decalcompref true false))

(event Custom|ShowSelectionDecal
  (bind _decalcompref (Variables|Default|GetDecalCompRef))
  (Rendering|SetVisibility _decalcompref true false)
  (Development|SetHiddeninGame _decalcompref false false))

(event EventBeginPlay
  (bind _indicatorradius (Variables|Default|GetIndicatorRadius))
  (bind _returnvalue (Game|AddComponentbyClass (Components|GetOwner) "/Script/Engine.DecalComponent" false (Math|Transform|MakeTransform "0, 0, 0" "90.000000, 0, 0" "1.000000,1.000000,1.000000")))
  (Variables|Default|SetDecalCompRef _returnvalue)
  (Rendering|Components|Decal|SetDecalMaterial (Variables|Default|GetDecalCompRef) "/Game/MyFirstRTS/Core/Building/MI_SelectionIndicator.MI_SelectionIndicator")
  (CallFunction|HideSelectionDecal)
  (Transformation|SetRelativeScale3D (Variables|Default|GetDecalCompRef) (Math|Vector|MakeVector 128.0 (/ _indicatorradius (.y (Variables|/Script/Engine.DecalComponent|GetDecalSize (Variables|Default|GetDecalCompRef)))) (/ _indicatorradius (.z (Variables|/Script/Engine.DecalComponent|GetDecalSize (Variables|Default|GetDecalCompRef))))))
  (Transformation|SetRelativeLocation (Variables|Default|GetDecalCompRef) (Variables|Default|GetIndicatorOffset) false false))