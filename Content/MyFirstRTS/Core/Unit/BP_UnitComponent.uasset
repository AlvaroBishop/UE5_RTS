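; BP_UnitComponent is an actor component that gives its owning RTS unit health, team attitude, click selection and a unit state.
; On BeginPlay it adds a team-colored health bar widget component to the owner and binds the owner's click and damage events.
; Clicking a friendly unit adds it to PC_MyFirstRTS's selection list.
; Damage updates the bar; at zero health the owner is destroyed, decrementing BP_GameManager's unit count if friendly.
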(event Custom|OnOwnerClicked
  (params (TouchedActor :type Actor%20Object%20Reference) (ButtonPressed :type Key%20Structure :default "None"))
  (if (Utilities|Enum|Equal(Enum) (Variables|Default|GetTeamAttitude) "Friendly")
    (CallFunction|AddUnittoSelectionList)))

(event Custom|AddUnitToSelectionList
  (bind _aspc_my_first_rts (Utilities|Casting|CastToPC_MyFirstRTS (Game|GetPlayerController 0)))
  (Default|AddActorSelectedtoList _aspc_my_first_rts (Components|GetOwner)))

(event Custom|OnOwnerTakeAnyDamage
  (params (DamagedActor :type Actor%20Object%20Reference) (Damage :type Float%20%28single-precision%29) (DamageType :type Damage%20Type%20Object%20Reference) (InstigatedBy :type Controller%20Object%20Reference) (DamageCauser :type Actor%20Object%20Reference))
  (Variables|Default|SetHealth (Math|Float|Max(Float) (- (Variables|Default|GetHealth) Damage) 0.0))
  (CallFunction|UpdateHealthBar)
  (if (<= (Variables|Default|GetHealth) 0.0)
    (if (Utilities|Enum|Equal(Enum) (Variables|Default|GetTeamAttitude) "Friendly")
      (bind _returnvalue (Actor|GetActorOfClass "/Game/PaulTestArea/BP_GameManager.BP_GameManager_C"))
      (Math|Integer|DecrementInt (Variables|/Game/PaulTestArea/BP_GameManager.BP_GameManager_C|GetCurrentNumberOfUnits _returnvalue)
        (:%20%20
          _)))
    (Actor|DestroyActor DamagedActor)))

(event EventBeginPlay
  (Utilities|FlowControl|Sequence
    (:then_0
      (bind _returnvalue (Game|AddComponentbyClass (Components|GetOwner) "/Game/MyFirstRTS/Core/Unit/BP_HealthBarWidgetComponent.BP_HealthBarWidgetComponent_C" false (Math|Transform|MakeTransform (Variables|HealthBar|GetHealthBarRelativeLocation) "0, 0, 0" "1.000000,1.000000,1.000000")))
      (Class|WidgetComponent|SetDrawSize _returnvalue (Variables|HealthBar|GetHealthBarDrawSize))
      (Default|UpdateHealthBarColor _returnvalue (Utilities|Select :Index (Variables|Default|GetTeamAttitude) :Friendly "(R=0.000000,G=0.500000,B=1.000000,A=1.000000)" :Neutral "(R=1.000000,G=0.911144,B=0.000000,A=1.000000)" :Hostile "(R=1.000000,G=0.000000,B=0.000000,A=1.000000)"))
      (CallFunction|UpdateHealthBar))
    (:then_1
      (EventDispatchers|BindEventtoOnClicked (Components|GetOwner) (EventDispatchers|CreateEvent :!event Custom|OnOwnerClicked))
      (EventDispatchers|BindEventtoOnTakeAnyDamage (Components|GetOwner) (EventDispatchers|CreateEvent :!event Custom|OnOwnerTakeAnyDamage)))))

(fn HandleNewUnitState
  (params (NewUnitState :type E_UnitStates%20Enum :default "NewEnumerator0"))
  (bind _output_get (Variables|Default|SetUnitState NewUnitState))
  (Default|CallOnEnterNewState _output_get))

(fn UpdateHealthBar
  (bind _returnvalue (Components|GetOwner))
  (bind _returnvalue_2 (Actor|GetComponentbyClass _returnvalue "/Game/MyFirstRTS/Core/Unit/BP_HealthBarWidgetComponent.BP_HealthBarWidgetComponent_C"))
  (Utilities|IsValid _returnvalue_2
    (:Is%20Valid
      (Default|UpdateHealthBar _returnvalue_2 (/ (Variables|Default|GetHealth) (Variables|Default|GetHealthMax))))
    (:Is%20Not%20Valid
      (Development|PrintString "Unit Component: No Healthbar component valid"))))